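; BP_Mushroom is a ranged enemy character that fires projectiles at the player.
; Each tick it flips to face the player along X until dead.
; Overlapping its attack box starts a looping, never-cleared timer that triggers attack animations; SpawnProjectile fires from its head.
; Damage updates a widget health bar, knocks it away from the causer and plays hit or death states, with delayed destruction on death.
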(event OnComponentBeginOverlap(AttackBoxTrigger)
  (params (OverlappedComponent :type Primitive%20Component%20Object%20Reference) (OtherActor :type Actor%20Object%20Reference) (OtherComp :type Primitive%20Component%20Object%20Reference) (OtherBodyIndex :type Integer) (bFromSweep :type Boolean) (SweepResult :type Hit%20Result%20Structure%20%28by%20ref%29))
  ;[1 1 1] If Player Overlap AttackBoxTrigger, Plays Attack Anim. On 7th Frame via AN Projectile Spawns
  (if (== OtherActor (Game|GetPlayerCharacter 0))
    (Utilities|Time|SetTimerbyEvent (delegate Custom|AttackMushroom) 0.7 true)))

(event Custom|HandleRotation
  ;[1 1 1] Rotation toward Player
  (if (not (Variables|DoNotEdit|GetIsDead?))
    (if (< (.x (Math|Vector|GetUnitDirection(Vector) (Transformation|GetActorLocation (Game|GetPlayerCharacter 0)) (Transformation|GetActorLocation))) 0.0)
      (Transformation|SetActorRotation "0, 0, 0")
      (else
        (Transformation|SetActorRotation "0.000000,180.000000,1.000000")))))

(event Custom|AttackMushroom
  ;[1 1 1] If Player Overlap AttackBoxTrigger, Plays Attack Anim. On 7th Frame via AN Projectile Spawns
  (if (not (or (Variables|DoNotEdit|GetIsDead?) (AI|Components|NavMovement|IsFalling (Variables|Character|GetCharacterMovement))))
    (Class|PaperZDAnimInstance|JumptoNode (Variables|/Script/PaperZD.PaperZDAnimationComponent|GetAnimInstance (Variables|Default|GetAnimationComponent)) (Variables|Edit|GetJump%20Node%20Attack) (Variables|Edit|GetState%20Machine%20Name))))

(event Custom|SpawnProjectile
  ;[1 1 1] If Player Overlap AttackBoxTrigger, Plays Attack Anim. On 7th Frame via AN Projectile Spawns
  ;;[1 1 1] Spawn Projectiles in Mushroom Head (SpawnPoint)
  (Game|SpawnActorfromClass (Variables|Edit|GetProjectiles) (Math|Transform|MakeTransform (Transformation|GetWorldLocation (Variables|Default|GetSpawnPoint)) (Transformation|GetActorRotation) "1.000000,1.000000,1.000000") "Undefined" "MultiplyWithRoot" 0 0))

(event EventTick
  (params (DeltaSeconds :type Float%20%28single-precision%29))
  ;[1 1 1] Every frame check Rotation of Enemy to the Player
  (CallFunction|HandleRotation))

(event Game|Damage|EventAnyDamage
  (params (Damage :type Float%20%28single-precision%29) (DamageType :type Damage%20Type%20Object%20Reference) (InstigatedBy :type Controller%20Object%20Reference) (DamageCauser :type Actor%20Object%20Reference))
  ;[1 1 1] if Enemy get Damaged while he is not faced Warrior, he will turn around
  (Variables|Edit|SetHealth (- (Variables|Edit|GetHealth) Damage))
  (Default|UpdateHealthBar (Variables|DoNotEdit|GetWBP%20Ranged%20Enemy%20Health%20Bar))
  (Variables|DoNotEdit|SetEnemyDamaged? true)
  (if (<= (Variables|Edit|GetHealth) 0.0)
    (Class|PaperZDAnimInstance|JumptoNode (Variables|/Script/PaperZD.PaperZDAnimationComponent|GetAnimInstance (Variables|Default|GetAnimationComponent)) (Variables|Edit|GetJump%20Node%20Death) (Variables|Edit|GetState%20Machine%20Name))
    (Variables|DoNotEdit|SetIsDead? true)
    ;[1 1 1] Makes EnemyHealthBar invisible after Death
    (Rendering|SetVisibility (Variables|Default|GetWidget) false false)
    (Collision|SetCollisionProfileName (Variables|Default|GetCapsuleComponent) "OverlapOnlyPawn" true :!class /Script/Engine.PrimitiveComponent)
    (Utilities|FlowControl|Delay 5.0)
    (Actor|DestroyActor)
    (else
      ;[1 1 1] Bounce (push) Enemy in oposite Direction
      (Character|LaunchCharacter (Math|Vector|MakeVector (* (select (< (.x (Math|Vector|GetUnitDirection(Vector) (Transformation|GetActorLocation DamageCauser) (Transformation|GetActorLocation))) 0.0) 1.0 -1.0) -6e+02) 0.0 1.5e+02) true true)
      (Class|PaperZDAnimInstance|JumptoNode (Variables|/Script/PaperZD.PaperZDAnimationComponent|GetAnimInstance (Variables|Default|GetAnimationComponent)) (Variables|Edit|GetJump%20Node%20Damaged) (Variables|Edit|GetState%20Machine%20Name))
      ;[1 1 1] Makes EnemyHealthBar visible after damage
      (Rendering|SetVisibility (Variables|Default|GetWidget) true false)
      (Utilities|FlowControl|RetriggerableDelay 1.0)
      (Variables|DoNotEdit|SetEnemyDamaged? false))))

(event EventBeginPlay
  (Variables|DoNotEdit|SetMaxHealth (Variables|Edit|GetHealth))
  ;[1 1 1] Initialization between BP and Widget
  (bind _aswbp_ranged_enemy_health_bar (Utilities|Casting|CastToWBP_RangedEnemyHealthBar (UserInterface|GetWidget (Variables|Default|GetWidget))))
  (bind _output_get (Variables|DoNotEdit|SetWBP%20Ranged%20Enemy%20Health%20Bar _aswbp_ranged_enemy_health_bar))
  (Variables|/Game/Blueprints/UI/Widgets/WBP_RangedEnemyHealthBar.WBP_RangedEnemyHealthBar_C|SetMushroomReference _output_get self))

(fn ConstructionScript)