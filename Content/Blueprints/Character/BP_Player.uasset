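; BP_Player is the 2D platformer player character, with Enhanced Input movement, jump, dash, wall slide and melee attack.
; Movement direction flips control rotation, while actions jump to Locomotion animation nodes.
; Dashes briefly cancel gravity when airborne, and hits on "Wall"-tagged actors open a retriggerable slide window for wall jumps.
; An animation-timed line trace damages pawns, and damage taken lowers Health and updates HUD hearts, with key 1 self-damaging.
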(event Custom|Attack
  (bind _returnvalue (Transformation|GetActorLocation))
  ;[1 1 1] 100u in front of Player is an Attacking Zone. Attacks Enemies (other Pawns), ignores myself
  (bind _outhit (Collision|LineTraceForObjects _returnvalue (+ _returnvalue (* (Transformation|GetActorForwardVector) (Math|Vector|MakeVector 1e+02 0.0 0.0))) (Utilities|Array|MakeArray "ObjectTypeQuery3") false (Utilities|Array|MakeArray (Game|GetPlayerCharacter 0)) "ForDuration"))
  ;[1 1 1] Comment
  (Game|Damage|ApplyDamage (.HitActor (Collision|BreakHitResult _outhit)) 1.0 0 self))

(event Input|EnhancedActionEvents|EnhancedInputActionIA_Jump
  (params (ActionValue :type Boolean) (ElapsedSeconds :type Float%20%28double-precision%29) (TriggeredSeconds :type Float%20%28double-precision%29) (InputAction :type Input%20Action%20Object%20Reference :default "/Game/Input/Actions/IA_Jump.IA_Jump"))
  (:Started
    ;[1 1 1] Bounce (push) Char off the wall if press Jump during WallSlide
    (if (Variables|Default|GetSlideWall?)
      (Character|LaunchCharacter (Math|Vector|MakeVector (* (.x (Transformation|GetActorForwardVector)) -1e+03) 0.0 7.5e+02) true true)
      (else
        (Character|Jump))))
  (:Completed
    (Character|StopJumping)))

(event Input|EnhancedActionEvents|EnhancedInputActionIA_Move
  (params (ActionValue :type Float%20%28double-precision%29) (ElapsedSeconds :type Float%20%28double-precision%29) (TriggeredSeconds :type Float%20%28double-precision%29) (InputAction :type Input%20Action%20Object%20Reference :default "/Game/Input/Actions/IA_Move.IA_Move"))
  (:Triggered
    ;[1 1 1] Movements R/L and Setting of MoveRight? var
    ;;[1 1 1] Setting for var MoveRight?. Whithout this part work perfect
    (if (> ActionValue 0.0)
      (Variables|Default|SetMoveRight? true)
      (elif (< ActionValue 0.0)
        (Variables|Default|SetMoveRight? false)))
    (Pawn|Input|AddMovementInput "1.000000,0.000000,0.000000" ActionValue false)))

(event Input|EnhancedActionEvents|EnhancedInputActionIA_Dash
  (params (ActionValue :type Boolean) (ElapsedSeconds :type Float%20%28double-precision%29) (TriggeredSeconds :type Float%20%28double-precision%29) (InputAction :type Input%20Action%20Object%20Reference :default "/Game/Input/Actions/IA_Dash.IA_Dash"))
  (:Started
    ;[1 1 1] Push the Warrior on +-3000. TimeDelay beetween Dashes 0.3sec. Change Gravity for Dash during Jump/Fall. Play Anim from JumpDash Node.
    (Utilities|FlowControl|DoOnce false :!label _label
      (:Completed
        (Class|PaperZDAnimInstance|JumptoNode (Variables|/Script/PaperZD.PaperZDAnimationComponent|GetAnimInstance (Variables|Default|GetAnimationComponent)) "JumpDash" "Locomotion")
        (if (AI|Components|NavMovement|IsFalling (Variables|Character|GetCharacterMovement))
          (Variables|/Script/Engine.CharacterMovementComponent|SetGravityScale (Variables|Character|GetCharacterMovement) 0.0))
        (Character|LaunchCharacter (Math|Vector|MakeVector (select (Variables|Default|GetMoveRight?) 3e+03 -3e+03) 0.0 0.0) true true)
        (Utilities|FlowControl|Delay 0.3)
        (Variables|/Script/Engine.CharacterMovementComponent|SetGravityScale (Variables|Character|GetCharacterMovement) 1.0)
        (goto _label Reset)))))

(event Input|EnhancedActionEvents|EnhancedInputActionIA_Attack
  (params (ActionValue :type Boolean) (ElapsedSeconds :type Float%20%28double-precision%29) (TriggeredSeconds :type Float%20%28double-precision%29) (InputAction :type Input%20Action%20Object%20Reference :default "/Game/Input/Actions/IA_Attack.IA_Attack"))
  (:Started
    ;[1 1 1] Play AttackAnim via JumpNode. Posible Once at the time. Repeat posiblle after 0.4sec. Attack triggers on 5th Frame of the AttackAnim with AnimNode_Attack
    (Utilities|FlowControl|DoOnce false :!label _label
      (:Completed
        (Class|PaperZDAnimInstance|JumptoNode (Variables|/Script/PaperZD.PaperZDAnimationComponent|GetAnimInstance (Variables|Default|GetAnimationComponent)) "JumpAttack" "Locomotion")
        (Utilities|FlowControl|Delay 0.4)
        (goto _label Reset)))))

(event EventBeginPlay
  ;[1 1 1] Initialization of the Players Input
  (bind _asplayer_controller (Utilities|Casting|CastToPlayerController (Pawn|GetController)))
  (Utilities|IsValid (PlayerController|LocalPlayerSubsystems|GetEnhancedInputLocalPlayerSubsystem _asplayer_controller)
    (:Is%20Valid
      (Input|AddMappingContext (PlayerController|LocalPlayerSubsystems|GetEnhancedInputLocalPlayerSubsystem _asplayer_controller) "/Game/Input/IMC_FullPlatformer.IMC_FullPlatformer" 0 "(bIgnoreAllPressedKeysUntilRelease=True,bForceImmediately=False)")
      (bind _returnvalue (UserInterface|CreateWidget "/Game/Blueprints/UI/Widgets/WBP_PlayerHUD.WBP_PlayerHUD_C"))
      (bind _output_get (Variables|Default|SetPlayerHUDRef _returnvalue))
      (UserInterface|Viewport|AddtoViewport _output_get 0))))

(event Collision|EventActorBeginOverlap
  (params (OtherActor :type Actor%20Object%20Reference)))

(event EventTick
  (params (DeltaSeconds :type Float%20%28single-precision%29))
  (bind _returnvalue (Pawn|GetController))
  (bind _returnvalue_2 (Pawn|GetController))
  ;[1 1 1] Rotation of Char depends of R/L (+- on X axis)
  (Math|Float|CompareFloat (.x (Variables|/Script/Engine.MovementComponent|GetVelocity (Variables|Character|GetCharacterMovement))) 0.0
    (:>
      ;;[1 1 1] if movement velocity >0, then no Rotation
      (Utilities|IsValid _returnvalue_2 :!label _label
        (:Is%20Valid
          (Pawn|SetControlRotation _returnvalue_2 (Math|Rotator|MakeRotator 0.0 0.0 0.0)))))
    (:==
      (if (Variables|Default|GetMoveRight?)
        (goto _label)
        (else
          ;;[1 1 1] if movement velocity <0, then 180ZRotation
          (Utilities|IsValid _returnvalue :!label _label_2
            (:Is%20Valid
              (Pawn|SetControlRotation _returnvalue (Math|Rotator|MakeRotator 0.0 0.0 1.8e+02)))))))
    (:<
      (goto _label_2))))

(event Collision|EventHit
  (params (MyComp :type Primitive%20Component%20Object%20Reference) (Other :type Actor%20Object%20Reference) (OtherComp :type Primitive%20Component%20Object%20Reference) (bSelfMoved :type Boolean) (HitLocation :type Vector :default "0, 0, 0") (HitNormal :type Vector :default "0, 0, 0") (NormalImpulse :type Vector :default "0, 0, 0") (Hit :type Hit%20Result%20Structure%20%28by%20ref%29))
  (bind _sprite (Variables|Default|GetSprite))
  (bind _sprite_2 (Variables|Default|GetSprite))
  (bind _relativelocation (Variables|/Script/Engine.SceneComponent|GetRelativeLocation _sprite))
  (bind _relativelocation_2 (Variables|/Script/Engine.SceneComponent|GetRelativeLocation _sprite_2))
  ;[1 1 1] Jump on the objects tagged 'Wall'. Anim Play from JumpWallSlide Node. Sprite RelativeLocation moves 42 during WallSlide, because of displaced sprites of Flipbook
  (if (and (Actor|ActorHasTag Other "Wall") (AI|Components|NavMovement|IsFalling (Variables|Character|GetCharacterMovement)))
    (Variables|Default|SetSlideWall? true)
    (Class|PaperZDAnimInstance|JumptoNode (Variables|/Script/PaperZD.PaperZDAnimationComponent|GetAnimInstance (Variables|Default|GetAnimationComponent)) "JumpWallSlide" "Locomotion")
    (Transformation|SetRelativeLocation _sprite_2 (Math|Vector|MakeVector 42.0 (.y _relativelocation_2) (.z _relativelocation_2)) false false)
    (Utilities|FlowControl|RetriggerableDelay 0.1)
    (Variables|Default|SetSlideWall? false)
    (Transformation|SetRelativeLocation _sprite (Math|Vector|MakeVector 0.0 (.y _relativelocation) (.z _relativelocation)) false false)))

(event Game|Damage|EventAnyDamage
  (params (Damage :type Float%20%28single-precision%29) (DamageType :type Damage%20Type%20Object%20Reference) (InstigatedBy :type Controller%20Object%20Reference) (DamageCauser :type Actor%20Object%20Reference))
  ;[1 1 1] - Damage, set -1 to HealthPoints
  (Variables|Default|SetHealth (- (Variables|Default|GetHealth) Damage))
  ;[1 1 1] Check Array, Without 0
  (for _index (range 1 (Math|Float|Truncate Damage))
    ;[1 1 1] - Heart in HUD if Damaged
    (Default|PlayerDamaged (Variables|Default|GetPlayerHUDRef))))

(event Input|KeyboardEvents|1
  (params (Key :type Key%20Structure :default "None"))
  (:Pressed
    (Game|Damage|ApplyDamage self 1.0 0 0)))

(fn ConstructionScript)