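; BP_Skeleton is a patrolling enemy character that walks back and forth along the world X axis.
; Each Tick, it moves by MovementDirection and flips its rotation to match that sign.
; A 100-unit forward trace detects world objects and pawns, ignoring the player and drawing debug lines.
; On a hit, a DoOnce-gated sequence stops it, waits WaitTime, restores speed and reverses direction.
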(event Custom|HandleMovement
  (bind _returnvalue (Transformation|GetActorLocation))
  ;[1 1 1] Just Movement straight
  (Pawn|Input|AddMovementInput "1.000000,0.000000,0.000000" (Variables|Default|GetMovementDirection) false)
  ;[1 1 1] Turn in front of walls, etc world, other Enemies. Ignores Player
  (bind _returnvalue_2 (Collision|LineTraceForObjects _returnvalue (+ _returnvalue (* (Transformation|GetActorForwardVector) (Math|Vector|MakeVector 1e+02 0.0 0.0))) (Utilities|Array|MakeArray "ObjectTypeQuery1" "ObjectTypeQuery2" "ObjectTypeQuery3") false (Utilities|Array|MakeArray (Game|GetPlayerCharacter 0)) "ForDuration"))
  (if _returnvalue_2
    (Utilities|FlowControl|DoOnce false :!label _label
      (:Completed
        ;[1 1 1] Enemy Stops before an obstacle
        (Variables|/Script/Engine.CharacterMovementComponent|SetMaxWalkSpeed (Variables|Character|GetCharacterMovement) 0.0)
        ;[1 1 1] How long it takes Enemy to turn Around
        (Utilities|FlowControl|Delay (Variables|Default|GetWaitTime))
        (Variables|/Script/Engine.CharacterMovementComponent|SetMaxWalkSpeed (Variables|Character|GetCharacterMovement) (Variables|Default|GetMax%20Walk%20Speed))
        ;[1 1 1] Turn in the opposite direction
        (Variables|Default|SetMovementDirection (* (Variables|Default|GetMovementDirection) -1.0))
        (goto _label Reset)))))

(event Custom|HandleRotation
  ;[1 1 1] Sprite Rotation depends on +- X of MovementDirection
  (if (> (Variables|Default|GetMovementDirection) 0.0)
    (Transformation|SetActorRotation "0, 0, 0")
    (else
      (Transformation|SetActorRotation "0.000000,180.000000,0.000000"))))

(event EventBeginPlay
  ;[1 1 1] Set Skeleton's Max Speed (here and in HandleMovement function)
  (Variables|/Script/Engine.CharacterMovementComponent|SetMaxWalkSpeed (Variables|Character|GetCharacterMovement) (Variables|Default|GetMax%20Walk%20Speed)))

(event Collision|EventActorBeginOverlap
  (params (OtherActor :type Actor%20Object%20Reference)))

(event EventTick
  (params (DeltaSeconds :type Float%20%28single-precision%29))
  (CallFunction|HandleRotation)
  (CallFunction|HandleMovement))

(fn ConstructionScript)