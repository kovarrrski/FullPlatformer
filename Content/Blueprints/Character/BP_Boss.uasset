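; Boss character that chases and faces player 0 along the world X axis.
; Each Tick snaps its rotation between two opposite facings based on which side the player is on, unless IsDead is set.
; It then adds X movement input scaled by the normalized direction to the player, stopping inside a small X dead zone.
; The movement is not gated by IsDead.
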(event Custom|HandleRotation
  ;[1 1 1] Rotation toward Player
  (if (not (Variables|Default|GetIsDead?))
    (if (< (.x (Math|Vector|GetUnitDirection(Vector) (Transformation|GetActorLocation (Game|GetPlayerCharacter 0)) (Transformation|GetActorLocation))) 0.0)
      (Transformation|SetActorRotation "0, 0, 0")
      (else
        (Transformation|SetActorRotation "0.000000,180.000000,1.000000")))))

(event EventBeginPlay)

(event Collision|EventActorBeginOverlap
  (params (OtherActor :type Actor%20Object%20Reference)))

(event EventTick
  (params (DeltaSeconds :type Float%20%28single-precision%29))
  (bind _returnvalue (Transformation|GetActorLocation))
  (bind _returnvalue_2 (Game|GetPlayerCharacter 0))
  (bind _returnvalue_3 (Transformation|GetActorLocation _returnvalue_2))
  (bind _returnvalue_4 (- _returnvalue_3 _returnvalue))
  (CallFunction|HandleRotation)
  ;[1 1 1] If less than |450|uu till Player - boss will rotate
  (if (not (< (Math|Float|Absolute(Float) (.x _returnvalue_4)) 5.0))
    (Pawn|Input|AddMovementInput "1.000000,0.000000,0.000000" (.x (Math|Vector|Normalize (Math|Vector|MakeVector (.x _returnvalue_4) (.y _returnvalue_4) (.z _returnvalue_4)))) false)))

(fn ConstructionScript)