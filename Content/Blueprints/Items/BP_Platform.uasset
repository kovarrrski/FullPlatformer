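; BP_Platform is a 2D one-way platform that the player can jump through.
; Its Paper sprite starts with no collision, and a Box trigger enables query and physics collision while the player character overlaps it.
; When the player leaves the Box, collision switches off again so the platform can be passed through once more.
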(event OnComponentBeginOverlap(Box)
  (params (OverlappedComponent :type Primitive%20Component%20Object%20Reference) (OtherActor :type Actor%20Object%20Reference) (OtherComp :type Primitive%20Component%20Object%20Reference) (OtherBodyIndex :type Integer) (bFromSweep :type Boolean) (SweepResult :type Hit%20Result%20Structure%20%28by%20ref%29))
  ;[1 1 1] When Player leave Platform, it become without Collision. So Player can jump throu Platform again
  (if (== OtherActor (Game|GetPlayerCharacter 0))
    (Collision|SetCollisionEnabled (Variables|Default|GetPaperSprite) "QueryAndPhysics")))

(event OnComponentEndOverlap(Box)
  (params (OverlappedComponent :type Primitive%20Component%20Object%20Reference) (OtherActor :type Actor%20Object%20Reference) (OtherComp :type Primitive%20Component%20Object%20Reference) (OtherBodyIndex :type Integer))
  (if (== OtherActor (Game|GetPlayerCharacter 0))
    (Collision|SetCollisionEnabled (Variables|Default|GetPaperSprite) "NoCollision")))

(event EventBeginPlay
  ;[1 1 1] When Player leave Platform, it become without Collision. So Player can jump throu Platform again
  (Collision|SetCollisionEnabled (Variables|Default|GetPaperSprite) "NoCollision"))

(fn ConstructionScript)