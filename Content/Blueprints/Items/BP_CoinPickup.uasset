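; BP_CoinPickup is a coin that plays a sound and increments the player's coin count when BP_Player overlaps its sphere.
; Below 100, it saves to slot "1" with saved Coins set to zero rather than the new count, updates the HUD and destroys itself.
; At exactly 100, it only zeroes both counts, leaving the actor in place.
; The intended extra-life logic is disconnected and never runs.
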(event OnComponentBeginOverlap(Sphere)
  (params (OverlappedComponent :type Primitive%20Component%20Object%20Reference) (OtherActor :type Actor%20Object%20Reference) (OtherComp :type Primitive%20Component%20Object%20Reference) (OtherBodyIndex :type Integer) (bFromSweep :type Boolean) (SweepResult :type Hit%20Result%20Structure%20%28by%20ref%29))
  (bind _asbp_player (Utilities|Casting|CastToBP_Player OtherActor))
  (bind _output_get (Variables|Default|SetBP%20Player _asbp_player))
  (Audio|PlaySoundatLocation "/Game/Sounds/SC_RandomCoin.SC_RandomCoin" (Transformation|GetActorLocation) "0, 0, 0" 1.0 1.0 0.0 0 0 0 0)
  ;[1 1 1] if player pick up coin, if its #100 coin - player get +1Live (head). And if it is not coin #100 - player get +1 coin, and it adds to the screen
  (if (== (Variables|/Game/Blueprints/Character/BP_Player.BP_Player_C|GetCoins _output_get) 1e+02)
    (Variables|/Game/Blueprints/Character/BP_Player.BP_Player_C|SetCoins (Variables|Default|GetBP%20Player) 0.0)
    (Variables|/Game/Blueprints/BP_SaveGame.BP_SaveGame_C|SetCoins (Variables|/Game/Blueprints/Character/BP_Player.BP_Player_C|GetBP%20Save%20Game (Variables|Default|GetBP%20Player)) 0.0)
    (else
      (Variables|/Game/Blueprints/Character/BP_Player.BP_Player_C|SetCoins (Variables|Default|GetBP%20Player) (+ (Variables|/Game/Blueprints/Character/BP_Player.BP_Player_C|GetCoins (Variables|Default|GetBP%20Player)) 1.0))
      ;;[1 1 1] Coins Saving
      (Variables|/Game/Blueprints/BP_SaveGame.BP_SaveGame_C|SetCoins (Variables|/Game/Blueprints/Character/BP_Player.BP_Player_C|GetBP%20Save%20Game (Variables|Default|GetBP%20Player)) 0.0)
      (SaveGame|SaveGametoSlot (Variables|/Game/Blueprints/Character/BP_Player.BP_Player_C|GetBP%20Save%20Game (Variables|Default|GetBP%20Player)) "1")
      (Default|UpdateCoins (Variables|/Game/Blueprints/Character/BP_Player.BP_Player_C|GetPlayerHUDRef (Variables|Default|GetBP%20Player)))
      (Actor|DestroyActor))))

(event EventBeginPlay)

(event Collision|EventActorBeginOverlap
  (params (OtherActor :type Actor%20Object%20Reference)))

(event EventTick
  (params (DeltaSeconds :type Float%20%28single-precision%29)))

(fn ConstructionScript)