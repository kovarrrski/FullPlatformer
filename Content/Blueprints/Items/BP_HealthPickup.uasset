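; BP_HealthPickup is a heart pickup that restores health to BP_Player on overlap with its HeartSphere.
; If the player is below max health, it adds one health, clamped between HealthToGive and MaxHealth, then destroys itself.
; It refreshes the HUD through ShowHeart, passing the truncated HealthToGive rather than the new health value.
; At full health the pickup stays in the world.
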(event OnComponentBeginOverlap(HeartSphere)
  (params (OverlappedComponent :type Primitive%20Component%20Object%20Reference) (OtherActor :type Actor%20Object%20Reference) (OtherComp :type Primitive%20Component%20Object%20Reference) (OtherBodyIndex :type Integer) (bFromSweep :type Boolean) (SweepResult :type Hit%20Result%20Structure%20%28by%20ref%29))
  (bind _asbp_player (Utilities|Casting|CastToBP_Player OtherActor))
  (bind _output_get (Variables|Default|SetBP%20Player _asbp_player))
  (if (not (== (Variables|/Game/Blueprints/Character/BP_Player.BP_Player_C|GetHealth _output_get) (Variables|/Game/Blueprints/Character/BP_Player.BP_Player_C|GetMaxHealth _output_get)))
    ;[1 1 1] Add 1 Heart after Overlapp, if Amount is not MaxHealth already
    (Variables|/Game/Blueprints/Character/BP_Player.BP_Player_C|SetHealth (Variables|Default|GetBP%20Player) (Math|Float|Clamp(Float) (+ (Variables|/Game/Blueprints/Character/BP_Player.BP_Player_C|GetHealth (Variables|Default|GetBP%20Player)) 1.0) (Variables|Default|GetHealthToGive) (Variables|/Game/Blueprints/Character/BP_Player.BP_Player_C|GetMaxHealth (Variables|Default|GetBP%20Player))))
    ;[1 1 1] Updates Heart Amount on the Screen/Widget
    (Default|ShowHeart (Variables|/Game/Blueprints/Character/BP_Player.BP_Player_C|GetPlayerHUDRef (Variables|Default|GetBP%20Player)) (Math|Float|Truncate (Variables|Default|GetHealthToGive)))
    (Actor|DestroyActor)))

(event EventBeginPlay)

(event Collision|EventActorBeginOverlap
  (params (OtherActor :type Actor%20Object%20Reference)))

(event EventTick
  (params (DeltaSeconds :type Float%20%28single-precision%29)))

(fn ConstructionScript)