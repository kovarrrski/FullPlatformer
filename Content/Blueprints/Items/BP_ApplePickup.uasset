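; BP_ApplePickup is an item pickup that gives the player apples on overlap.
; Its AppleSphere overlap event casts the other actor to BP_Player and, unless Apples already equals MaxApples, adds a fixed amount clamped to that maximum.
; It then refreshes the count through the player's HUD reference and destroys itself, so a full player leaves the pickup in the world.
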(event OnComponentBeginOverlap(AppleSphere)
  (params (OverlappedComponent :type Primitive%20Component%20Object%20Reference) (OtherActor :type Actor%20Object%20Reference) (OtherComp :type Primitive%20Component%20Object%20Reference) (OtherBodyIndex :type Integer) (bFromSweep :type Boolean) (SweepResult :type Hit%20Result%20Structure%20%28by%20ref%29))
  (bind _asbp_player (Utilities|Casting|CastToBP_Player OtherActor))
  (bind _output_get (Variables|Default|SetBP%20Player _asbp_player))
  (if (not (== (Variables|/Game/Blueprints/Character/BP_Player.BP_Player_C|GetApples _output_get) (Variables|/Game/Blueprints/Character/BP_Player.BP_Player_C|GetMaxApples _output_get)))
    ;[1 1 1] Add 5 Apples after Overlapp, if Amount is not MaxApples already
    (Variables|/Game/Blueprints/Character/BP_Player.BP_Player_C|SetApples (Variables|Default|GetBP%20Player) (Math|Integer|Clamp(Integer) (+ (Variables|/Game/Blueprints/Character/BP_Player.BP_Player_C|GetApples (Variables|Default|GetBP%20Player)) 5) 1 (Variables|/Game/Blueprints/Character/BP_Player.BP_Player_C|GetMaxApples (Variables|Default|GetBP%20Player))))
    ;[1 1 1] Updates Apple Amount on the Screen/Widget
    (Default|UpdateApples (Variables|/Game/Blueprints/Character/BP_Player.BP_Player_C|GetPlayerHUDRef (Variables|Default|GetBP%20Player)))
    (Actor|DestroyActor)))

(event EventBeginPlay)

(event Collision|EventActorBeginOverlap
  (params (OtherActor :type Actor%20Object%20Reference)))

(event EventTick
  (params (DeltaSeconds :type Float%20%28single-precision%29)))

(fn ConstructionScript)